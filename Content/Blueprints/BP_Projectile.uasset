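; Projectile actor that, on striking the paper player character, either takes coconuts from them or damages them.
; Box overlap sets a hit flag for any actor, then casts to BP_MyPaperCharacter.
; A player with enough coconuts loses a batch and is flagged as having given them; otherwise they take damage, and either way the projectile is destroyed.
; A Delay on Tick otherwise destroys it after a short lifetime.
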(event OnComponentBeginOverlap(Box)
  (params (OverlappedComponent :type Primitive%20Component%20Object%20Reference) (OtherActor :type Actor%20Object%20Reference) (OtherComp :type Primitive%20Component%20Object%20Reference) (OtherBodyIndex :type Integer) (bFromSweep :type Boolean) (SweepResult :type Hit%20Result%20Structure%20%28by%20ref%29))
  (Variables|Default|SetHasHitPlayer true)
  (bind _asbp_my_paper_character (Utilities|Casting|CastToBP_MyPaperCharacter OtherActor))
  (if (> (Variables|/Game/Blueprints/BP_MyPaperCharacter.BP_MyPaperCharacter_C|GetCoconut%20Count _asbp_my_paper_character) 4)
    (Variables|Default|SetHasCoconut true)
    (Variables|/Game/Blueprints/BP_MyPaperCharacter.BP_MyPaperCharacter_C|SetCoconut%20Count _asbp_my_paper_character (- (Variables|/Game/Blueprints/BP_MyPaperCharacter.BP_MyPaperCharacter_C|GetCoconut%20Count _asbp_my_paper_character) 4))
    (Variables|/Game/Blueprints/BP_MyPaperCharacter.BP_MyPaperCharacter_C|SetCoconutsGiven _asbp_my_paper_character true)
    (else
      (Class|MyPaperCharacter|TakeDamage _asbp_my_paper_character 1e+01)))
  (Actor|DestroyActor))

(event EventBeginPlay)

(event Collision|EventActorBeginOverlap
  (params (OtherActor :type Actor%20Object%20Reference)))

(event EventTick
  (params (DeltaSeconds :type Float%20%28single-precision%29))
  (Utilities|FlowControl|Delay 2.0)
  (Actor|DestroyActor))

(fn ConstructionScript)