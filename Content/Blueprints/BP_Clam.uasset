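; Clam actor that fires projectiles at spawn point until it becomes openable, then yields a pearl collectable.
; Tick drives Shoot, which stops spawning projectiles once the player has given coconuts, or stops shooting when a player-hitting shot reports a coconut.
; Either case sets OpenClam, letting a player overlap on the Box play the open flipbook and spawn the pearl once.
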(event OnComponentBeginOverlap(Box)
  (params (OverlappedComponent :type Primitive%20Component%20Object%20Reference) (OtherActor :type Actor%20Object%20Reference) (OtherComp :type Primitive%20Component%20Object%20Reference) (OtherBodyIndex :type Integer) (bFromSweep :type Boolean) (SweepResult :type Hit%20Result%20Structure%20%28by%20ref%29))
  (if (Variables|Default|GetOpenClam)
    (Utilities|Casting|CastToBP_MyPaperCharacter OtherActor)
    (Sprite|SetFlipbook (Variables|Default|GetRenderComponent) "/Game/Assets/FlipBooks/Clam_Open_FB.Clam_Open_FB")
    (Utilities|FlowControl|DoOnce false
      (:Completed
        (Game|SpawnActorfromClass "/Game/Blueprints/BP_Pearl_Collectable.BP_Pearl_Collectable_C" (Transformation|GetWorldTransform (Variables|Default|GetSpawnPosPearl)) "AlwaysSpawn" 0 0)))))

(event Custom|Shoot
  (if (Variables|Default|GetCanShoot)
    (bind _asbp_my_paper_character (Utilities|Casting|CastToBP_MyPaperCharacter (Game|GetPlayerCharacter 0)))
    (if (Variables|/Game/Blueprints/BP_MyPaperCharacter.BP_MyPaperCharacter_C|GetCoconutsGiven _asbp_my_paper_character)
      (Variables|Default|SetOpenClam true)
      (Sprite|SetFlipbook (Variables|Default|GetRenderComponent) "/Game/Assets/FlipBooks/clamIdle.clamIdle")
      (else
        (bind _returnvalue (Game|SpawnActorfromClass "/Game/Blueprints/BP_Projectile.BP_Projectile_C" (Transformation|GetWorldTransform (Variables|Default|GetSpawnPosProjectile)) "AlwaysSpawn" 0 0))
        (bind _output_get (Variables|Default|SetShot _returnvalue))
        (if (Variables|/Game/Blueprints/BP_Projectile.BP_Projectile_C|GetHasHitPlayer _output_get)
          (if (Variables|/Game/Blueprints/BP_Projectile.BP_Projectile_C|GetHasCoconut _output_get)
            (Variables|Default|SetCanShoot false)
            (Variables|Default|SetOpenClam true)
            (else
              (Variables|Default|SetCanShoot false)
              (Utilities|FlowControl|Delay 1.0)
              (Variables|Default|SetCanShoot true)))
          (Utilities|FlowControl|Delay 1.0))
        (Utilities|IsValid (Variables|Default|GetShot)
          (:Is%20Valid
            (Actor|DestroyActor (Variables|Default|GetShot))))))))

(event EventBeginPlay
  (Variables|Default|SetCanShoot true))

(event Collision|EventActorBeginOverlap
  (params (OtherActor :type Actor%20Object%20Reference)))

(event EventTick
  (params (DeltaSeconds :type Float%20%28single-precision%29))
  (CallFunction|Shoot))

(fn ConstructionScript)