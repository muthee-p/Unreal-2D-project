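; BP_Spring is an actor that endlessly toggles its Box component between a raised position and its starting relative location.
; On BeginPlay it caches that location, then two timelines, MoveUp and MoveDown, restart each other on finish.
; Their updates set fixed positions without interpolation or sweep, so the box snaps between the two rather than sliding, with the timelines only setting the timing.
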(event EventBeginPlay
  (Variables|Default|SetInitial%20Location (Variables|/Script/Engine.SceneComponent|GetRelativeLocation (Variables|Default|GetBox)))
  (Timeline|Move%20up Play
    (:Update
      (Transformation|SetRelativeLocation (Variables|Default|GetBox) (+ (Variables|Default|GetInitial%20Location) "0, 0,53.000000") false false))
    (:Finished
      (Timeline|Move%20Down PlayFromStart
        (:Update
          (Transformation|SetRelativeLocation (Variables|Default|GetBox) (Variables|Default|GetInitial%20Location) false false))
        (:Finished
          (Timeline|Move%20up PlayFromStart))))))

(event Collision|EventActorBeginOverlap
  (params (OtherActor :type Actor%20Object%20Reference)))

(event EventTick
  (params (DeltaSeconds :type Float%20%28single-precision%29)))

(fn ConstructionScript)