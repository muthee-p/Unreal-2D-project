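; Paper2D player character that carries items to matching slots, picks up collectables and drives the WB_PlayerHealth HUD.
; GrabDrop hides an overlapped item and shows its sprite or the mop; dropping on an empty parent of matching class transfers the sprite and destroys the item.
; Capsule overlaps update and destroy BI_Collectables actors; helper functions track coconuts, pearls and map.
; Tick's delayed timer update targets a newly created widget, not the displayed one.
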(event OnComponentBeginOverlap(CapsuleComponent)
  (params (OverlappedComponent :type Primitive%20Component%20Object%20Reference) (OtherActor :type Actor%20Object%20Reference) (OtherComp :type Primitive%20Component%20Object%20Reference) (OtherBodyIndex :type Integer) (bFromSweep :type Boolean) (SweepResult :type Hit%20Result%20Structure%20%28by%20ref%29))
  (if (Utilities|DoesObjectImplementInterface OtherActor "/Game/Blueprints/BI_Collectables.BI_Collectables_C")
    (Class|BICollectables|UpdateCountonWidget(Message) OtherActor)
    (Actor|DestroyActor OtherActor)))

(event Custom|GrabItem
  (bind _overlappingactors (Collision|GetOverlappingActors "/Game/Blueprints/BP_Carriable_Item.BP_Carriable_Item_C" :!class /Script/Engine.Actor))
  (bind _output (Utilities|Array|Get(acopy) _overlappingactors))
  ;[1 1 1] GrabItem
  (Variables|Default|SetisCarrying true)
  (bind _asbp_carriable_item (Utilities|Casting|CastToBP_Carriable_Item _output))
  (Utilities|IsValid _output
    (:Is%20Valid
      (if (== (Utilities|GetClass _output) "/Game/Blueprints/BP_Mop.BP_Mop_C")
        (Rendering|SetVisibility (Variables|Default|GetMop) true true)
        (else
          (Rendering|Components|Sprite|SetSprite (Variables|Default|Getcarried%20item) (Sprite|GetSprite (Variables|/Script/Paper2D.PaperSpriteActor|GetRenderComponent _asbp_carriable_item)))))
      (Variables|Default|SetGrabbed%20Sprite (Sprite|GetSprite (Variables|/Script/Paper2D.PaperSpriteActor|GetRenderComponent _asbp_carriable_item)))
      (Variables|Default|SetGrabbed%20Item _asbp_carriable_item)
      (Rendering|SetVisibility (Variables|/Script/Engine.Actor|GetRootComponent _output) false false))))

(event Custom|DropItem
  (bind _overlappingactors (Collision|GetOverlappingActors "/Game/Blueprints/BP_Carriable_Item_Parent.BP_Carriable_Item_Parent_C" :!class /Script/Engine.Actor))
  (bind _output (Utilities|Array|Get(acopy) _overlappingactors))
  ;[1 1 1] Drop Item
  (Variables|Default|SetisCarrying false)
  (bind _asbp_carriable_item_parent (Utilities|Casting|CastToBP_Carriable_Item_Parent _output))
  (if (== (Utilities|GetClass (Variables|/Game/Blueprints/BP_Carriable_Item.BP_Carriable_Item_C|GetParent (Variables|Default|GetGrabbed%20Item))) (Utilities|GetClass _output))
    (bind _output_get (Variables|Default|SetAs%20BP%20Carriable%20Item%20Parent _asbp_carriable_item_parent))
    (Utilities|IsValid (Sprite|GetSprite (Variables|/Game/Blueprints/BP_Carriable_Item_Parent.BP_Carriable_Item_Parent_C|GetChildSprite _output_get))
      (:Is%20Not%20Valid
        (Rendering|Components|Sprite|SetSprite (Variables|Default|Getcarried%20item) 0)
        (Rendering|SetVisibility (Variables|Default|GetMop) false true)
        (Rendering|Components|Sprite|SetSprite (Variables|/Game/Blueprints/BP_Carriable_Item_Parent.BP_Carriable_Item_Parent_C|GetChildSprite _output_get) (Variables|Default|GetGrabbed%20Sprite))
        (Actor|DestroyActor (Variables|Default|GetGrabbed%20Item))
        (Variables|/Game/Blueprints/BP_Carriable_Item_Parent.BP_Carriable_Item_Parent_C|SetisMatched (Variables|Default|GetAs%20BP%20Carriable%20Item%20Parent) true)))))

(event EventBeginPlay
  (bind _returnvalue (UserInterface|CreateWidget "/Game/Blueprints/UI/WB_PlayerHealth.WB_PlayerHealth_C"))
  (bind _output_get (Variables|Default|SetHeathWidget _returnvalue))
  (UserInterface|Viewport|AddtoViewport _output_get 0)
  (CallFunction|SetHealthonWidget)
  (Variables|Default|SetMap (Class|WidgetBlueprintLibrary|MakeBrushfromMaterial "/Engine/MaterialTemplates/VertexAnimation/AdvancedFlag.AdvancedFlag" 32 32)))

(event EventTick
  (params (DeltaSeconds :type Float%20%28single-precision%29))
  (Variables|Default|SetTime (- (Variables|Default|GetMax%20Time) DeltaSeconds))
  (Utilities|FlowControl|Delay 3e+01)
  (CallFunction|SetTimeronWidget))

(event EventUpdateHealthWidget
  (CallFunction|SetHealthonWidget))

(event Input|ActionEvents|InputActionGrabDrop
  (params (Key :type Key%20Structure :default "None"))
  (:Pressed
    (Variables|Default|GetGrabbed%20Item
      (:then
        (CallFunction|DropItem))
      (:else
        (CallFunction|GrabItem)))))

(fn ConstructionScript)

(fn SetHealthonWidget
  (Default|UpdateHealth (Variables|Default|GetHeathWidget) (Variables|Default|GetHealth) (Variables|Default|GetMaxHealth)))

(fn SetCoconutonWidget
  (if (< (Variables|Default|GetCoconut%20Count) 10)
    (Variables|Default|SetCoconut%20Count (+ (Variables|Default|GetCoconut%20Count) 1))))

(fn SetPearlCountonWidget
  (if (< (Variables|Default|GetPearlCount) 5)
    (Variables|Default|SetPearlCount (+ (Variables|Default|GetPearlCount) 1))))

(fn SetMapImageonWidget
  (Variables|Default|SetMap (Class|PaperSpriteBlueprintLibrary|MakeBrushfromSprite "/Game/Assets/Sprites/Island/Map_Half_folded_Sprite_0.Map_Half_folded_Sprite_0"))
  (Variables|Default|SetGotMap true))

(fn CheckGame)

(fn SetTimeronWidget
  (bind _returnvalue (UserInterface|CreateWidget "/Game/Blueprints/UI/WB_PlayerHealth.WB_PlayerHealth_C"))
  (Default|UpdateTimer _returnvalue))